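; Player character Blueprint for Lublin whose only active logic opens the pause menu with the F key.
; When the game is unpaused, F shows the cursor, adds the PauseMenuBase widget to the viewport and pauses the game.
; The widget is created on first use and cached in ReferenceTheFMenu.
; UI-only input focused on the menu is set only when that cached widget already exists, not on first creation.
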(event EventBeginPlay)

(event Collision|EventActorBeginOverlap
  (params (OtherActor :type Actor%20Object%20Reference)))

(event EventTick
  (params (DeltaSeconds :type Float%20%28single-precision%29)))

(event Input|KeyboardEvents|F
  (params (Key :type Key%20Structure))
  ;[1 1 1] Wlaczenie Menu
  (:Pressed
    (if (not (Game|IsGamePaused))
      (Variables|/Script/Engine.PlayerController|SetbShowMouseCursor (Game|GetPlayerController 0) true)
      (Utilities|IsValid (Variables|Default|GetReferenceTheFMenu)
        (:Is%20Valid
          (Input|SetInputModeUIOnly (Game|GetPlayerController 0) (Variables|Default|GetReferenceTheFMenu) "DoNotLock"))
        (:Is%20Not%20Valid
          (bind _returnvalue (UserInterface|CreateWidget "/Game/UserInterface/PauseMenu/PauseMenuBase.PauseMenuBase_C"))
          (bind _output_get (Variables|Default|SetReferenceTheFMenu _returnvalue))))
      (UserInterface|Viewport|AddtoViewport _output_get 0)
      (Game|SetGamePaused true))))

(fn ConstructionScript)